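; BP_CameraSpline is a rail camera that becomes the player's view at BeginPlay and tracks the third-person character.
; After a one-tick delay it finds BP_ThirdPersonCharacter and sets itself as player 0's view target.
; Each tick, FollowCamera eases with VInterpTo toward the spline point closest to the character, using a swept move, then rotates to look directly at them.
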(event EventBeginPlay
  (Utilities|FlowControl|DelayUntilNextTick)
  (bind _returnvalue (Actor|GetActorOfClass "/Game/ThirdPerson/Blueprints/BP_ThirdPersonCharacter.BP_ThirdPersonCharacter_C"))
  (Variables|Default|SetTargetToFollow _returnvalue)
  (Game|Player|SetViewTargetwithBlend (Game|GetPlayerController 0) self 0.0 "VTBlend_Linear" 0.0 false))

(event EventTick
  (params (DeltaSeconds :type Float%20%28single-precision%29))
  (bind _targettofollow (Variables|Default|GetTargetToFollow))
  (bind _followcamera (Variables|Default|GetFollowCamera))
  (bind _followcamera_2 (Variables|Default|GetFollowCamera))
  (bind _returnvalue (Transformation|GetActorLocation _targettofollow))
  (bind _returnvalue_2 (Transformation|GetWorldLocation _followcamera_2))
  (Utilities|IsValid _targettofollow
    (:Is%20Valid
      (Transformation|SetWorldLocation _followcamera (Math|Interpolation|VInterpTo _returnvalue_2 (Spline|FindLocationClosesttoWorldLocation (Variables|Default|GetSpline) _returnvalue "World") (Utilities|Time|GetWorldDeltaSeconds) 2.0) true false)
      (Transformation|SetWorldRotation _followcamera (Math|Rotator|FindLookatRotation _returnvalue_2 _returnvalue) false false))))

(fn ConstructionScript)